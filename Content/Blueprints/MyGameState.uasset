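; Game state that tracks joined and qualified players in a level and plays the preview camera sequence shortly after start.
; Joining players raise the qualification cap to the full player count, with a temporary set used to deduplicate both lists.
; Each qualification refreshes the counter widgets and shows that player a qualified screen.
; It then calls the game mode's MoveToLevel immediately, as the all-qualified check is disconnected.
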(event Custom|M_Update%20Qualification%20UIs
  (params (qualified_player :type BP%20Chara%20Popo%20Object%20Reference))
  ;[1 0.5445 0.2417] Update qualified counter, and display qualified UI if is winning player
  (bind _foundwidgets (Widget|GetAllWidgetsOfClass "/Game/UI/UI_qualification.UI_qualification_C" true))
  (for _array_element _foundwidgets
    (Default|CUpdateNumberOfQualified _array_element)
    (if (== (Pawn|GetController qualified_player) (Widget|GetOwningPlayer _array_element))
      (bind _returnvalue (UserInterface|CreateWidget "/Game/UI/UI_qualified.UI_qualified_C"))
      (UserInterface|Viewport|AddtoViewport _returnvalue 0))))

(event EventBeginPlay
  ;[1 1 1] When player loads the level, plays the cinematic camera animation
  (Utilities|FlowControl|Delay 1.0)
  (bind _returnvalue (Sequencer|Player|CreateLevelSequencePlayer "/Game/Levels/Doors/level_preview.level_preview"))
  (Sequencer|Player|Play _returnvalue :!class /Script/MovieScene.MovieSceneSequencePlayer))

(fn ConstructionScript)

(fn AddNewPlayer
  (params (New%20Player :type BP%20Chara%20Popo%20Object%20Reference%20%28by%20ref%29))
  (bind _temp_set (LocalVariables|Gettemp_set))
  ;[0.8839 0.3913 1] TODO: If Game did not start yet
  (if (>= (Variables|Default|Gettimer) 0.0)
    ;[0.8839 0.3913 1] Add Player to list of players
    (Utilities|Set|AddItems _temp_set (Variables|Default|Getplayers))
    (Utilities|Set|Add _temp_set New%20Player)
    (bind _result (Utilities|Set|ToArray _temp_set))
    (bind _output_get (Variables|Default|Setplayers _result))
    ;[0.8839 0.3913 1] And update the number of potential qualifications
    (Variables|Default|Setmax_qualified (Utilities|Array|Length _output_get))))

(fn AddQualifiedPlayer
  (params (Qualified%20player :type BP%20Chara%20Popo%20Object%20Reference%20%28by%20ref%29))
  (bind _temp_set (LocalVariables|Gettemp_set))
  ;[0.9717 0.6765 1] If there is still some places to qualify
  (if (< (Utilities|Array|Length (Variables|Default|Getqualified_players)) (Variables|Default|Getmax_qualified))
    (Utilities|Set|AddItems _temp_set (Variables|Default|Getqualified_players))
    (Utilities|Set|Add _temp_set Qualified%20player)
    (bind _result (Utilities|Set|ToArray _temp_set))
    (bind _output_get (Variables|Default|Setqualified_players _result))
    (Variables|Default|Setcurrent_n_qualified (Utilities|Array|Length _output_get))
    (CallFunction|MUpdateQualificationUIs Qualified%20player)
    (CallFunction|CheckNumberQualifiedandMove)))

(fn CheckNumberQualifiedandMove
  (bind _asmy_game_mode (Utilities|Casting|CastToMyGameMode (Game|GetGameMode)))
  (Default|MovetoLevel _asmy_game_mode))