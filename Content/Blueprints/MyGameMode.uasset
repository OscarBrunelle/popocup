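; Game mode that freezes players for a short countdown at level start and handles falls and level travel.
; BeginPlay seeds the GameState Timer, which Tick decrements, and blocks input through each PC_doors controller until a separate fixed Delay ends.
; PostLogin applies the current block state to joining players.
; Handle_fall moves players to a fixed placeholder location pending checkpoints, and MoveToLevel server-travels to Remember.
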(event Custom|Handle_fall
  (params (Player :type BP%20Chara%20Popo%20Object%20Reference))
  ;[1 1 1] Move player back to checkpoint if fall OOB
  (Development|PrintString "TODO: Sending back to last checkpoint")
  (Transformation|SetActorLocation Player "0, 0,1000.000000" false false))

(event Custom|DisablePlayersMovement
  ;[1 1 1] Disable players movement
  (CallFunction|TogglePlayersMovement true))

(event Custom|setTimerBlockMovement
  ;[1 1 1] When server loads the level, set the timer to 10s
  (bind _asmy_game_state (Utilities|Casting|CastToMyGameState (Game|GetGameState)))
  (Variables|/Game/Blueprints/MyGameState.MyGameState_C|Settimer _asmy_game_state 1e+01))

(event Custom|EnablePlayersMovement
  ;[1 1 1] Enable players movement
  (CallFunction|TogglePlayersMovement false))

(event EventBeginPlay
  ;[1 1 1] Blocking movements at the beginning
  (CallFunction|SetTimerBlockMovement)
  (CallFunction|DisablePlayersMovement)
  (Utilities|FlowControl|Delay 1e+01)
  (CallFunction|EnablePlayersMovement))

(event EventTick
  (params (DeltaSeconds :type Float%20%28single-precision%29))
  ;[1 1 1] Decrease the timer over time
  (bind _asmy_game_state (Utilities|Casting|CastToMyGameState (Game|GetGameState)))
  (Variables|/Game/Levels/Doors/GS_doors.GS_doors_C|Settimer _asmy_game_state (- (Variables|/Game/Levels/Doors/GS_doors.GS_doors_C|Gettimer _asmy_game_state) DeltaSeconds)))

(event EventOnLogout
  (params (ExitingController :type Controller%20Object%20Reference)))

(event EventPostLogin
  (params (NewPlayer :type Player%20Controller%20Object%20Reference))
  ;[1 1 1] Block player when connected TODO add a check to see if all connected
  (bind _aspc_doors (Utilities|Casting|CastToPC_doors NewPlayer))
  (Default|ToggleBlockMovement _aspc_doors (Variables|Default|GetPlayerMovementBlocked)))

(fn ConstructionScript)

(fn TogglePlayersMovement
  (params (blockMovement :type Boolean))
  ;[1 1 1] For each player
  (bind _output_get (Variables|Default|SetPlayerMovementBlocked blockMovement))
  (bind _asmy_game_state (Utilities|Casting|CastToMyGameState (Game|GetGameState)))
  (for _array_element (Variables|/Game/Levels/Doors/GS_doors.GS_doors_C|Getplayers _asmy_game_state)
    ;[1 1 1] Block or ignore movement input
    (bind _aspc_doors (Utilities|Casting|CastToPC_doors (Pawn|GetController _array_element)))
    (Default|ToggleBlockMovement _aspc_doors _output_get)))

(fn MovetoLevel
  (Development|ExecuteConsoleCommand "serverTravel Remember" 0))