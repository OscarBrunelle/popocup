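; Player controller that manages qualification UI screens and switches the player between UI-only and game-only input.
; On BeginPlay it blocks movement through UI-only input mode with a locked mouse and adds the qualification widget to the viewport.
; Custom events toggle the input mode and show the "Qualified !" widget when the player qualifies.
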(event Custom|Qualify%20player
  ;[1 1 1] Adds the "Qualified !" UI to the screen
  (bind _returnvalue (UserInterface|CreateWidget "/Game/UI/UI_qualified.UI_qualified_C"))
  (UserInterface|Viewport|AddtoViewport _returnvalue 0))

(event Custom|Add%20UI
  ;[1 1 1] Adds the Qualification UI to the screen
  (bind _returnvalue (UserInterface|CreateWidget "/Game/UI/UI_qualification.UI_qualification_C"))
  (UserInterface|Viewport|AddtoViewport _returnvalue 0))

(event Custom|ToggleBlockMovement
  (params (Block :type Boolean))
  (bind _self self)
  ;[1 1 1] Block or ignore movement input
  (if Block
    (Input|SetInputModeUIOnly _self 0 "LockAlways")
    (else
      (Input|SetInputModeGameOnly _self))))

(event EventBeginPlay
  (CallFunction|ToggleBlockMovement true)
  (CallFunction|AddUI))

(event EventTick
  (params (DeltaSeconds :type Float%20%28single-precision%29)))

(fn ConstructionScript)