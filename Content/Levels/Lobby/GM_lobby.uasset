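; Lobby game mode that holds joining players until the session is full, then moves them to the Game map.
; PostLogin records each player controller and compares the count to the session's connection count from GetSessionSettings.
; Once that count is reached, it waits briefly and runs a serverTravel console command, printing debug text along the way.
; Logout removes the exiting controller from the list but does not cancel a pending travel.
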(event EventBeginPlay)

(event EventTick
  (params (DeltaSeconds :type Float%20%28single-precision%29)))

(event EventPostLogin
  (params (NewPlayer :type Player%20Controller%20Object%20Reference))
  (Utilities|Array|AddUnique (Variables|Default|GetControllers) NewPlayer)
  (bind _numconnections (Class|AdvancedSessionsLibrary|GetSessionSettings)
    (:OnSuccess
      (if (>= (Utilities|Array|Length (Variables|Default|GetControllers)) _numconnections)
        (Development|PrintText "Moving")
        (Utilities|FlowControl|Delay 5.0)
        (Development|ExecuteConsoleCommand "serverTravel Game" 0)
        (Development|PrintText "Moved")
        (else
          (Development|PrintText "Not Moving"))))))

(event EventOnLogout
  (params (ExitingController :type Controller%20Object%20Reference))
  (bind _asplayer_controller (Utilities|Casting|CastToPlayerController ExitingController))
  (Utilities|Array|RemoveItem (Variables|Default|GetControllers) _asplayer_controller))

(fn ConstructionScript)